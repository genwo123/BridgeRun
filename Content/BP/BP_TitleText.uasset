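; BP_TitleText is a title text actor whose text render component continuously cycles through rainbow colors.
; Each Tick advances a ColorCycle value by scaled delta time and wraps it between 0 and 1, completing a loop about every ten seconds.
; That value becomes the hue of a fully saturated, full-brightness HSV color, which is converted to sRGB and applied to the text.
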(event EventBeginPlay
  (Variables|Default|SetColorCycle 0.0))

(event EventTick
  (params (DeltaSeconds :type Float%20%28single-precision%29))
  (bind _output_get (Variables|Default|SetColorCycle (.Remainder (Math|Float|Division(WholeandRemainder) (+ (Variables|Default|GetColorCycle) (* DeltaSeconds 0.1)) 1.0))))
  (Rendering|Components|TextRender|SetTextRenderColor (Variables|Default|GetTextRender) (Math|Conversions|ToColor(LinearColor) (Class|KismetMathLibrary|HSVtoRGB (* _output_get 3.6e+02) 1.0 1.0 1.0))))

(fn ConstructionScript)